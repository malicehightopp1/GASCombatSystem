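; Gameplay ability that staggers an AI-controlled character with a stun montage.
; On activation it halts movement, stops the AI controller's brain logic and plays AM_Stunned.
; When the montage completes, is interrupted or is cancelled, it ends the ability, then restores walking and restarts the brain unless the owner has the State.Dead tag.
; Non-AI avatars exit at the controller cast, before the montage or EndAbility.
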(event `self.K2_ActivateAbility`
  (bind _ascharacter (cast `Character` (`self.GetAvatarActorFromActorInfo`)))
  (`MovementComponent.StopMovementImmediately` (`Character.CharacterMovement` _ascharacter))
  (bind _asaicontroller (cast `AIController` (`Pawn.GetController` _ascharacter)))
  (bind _braincomponent (`AIController.BrainComponent` _asaicontroller))
  (`/Engine/EditorBlueprintResources/StandardMacros.IsValid` _braincomponent
    (:`Is Valid`
      (`BrainComponent.StopLogic` _braincomponent "\"Staggered\""))
    (:`Is Not Valid`
      _))
  (`AbilityTask_PlayMontageAndWait.CreatePlayMontageAndWaitProxy` "None" "/Game/_MyFiles/Characters/Player/Animations/AnimMontages/Stunned/AM_Stunned.AM_Stunned"
    (:`OnCompleted`
      _)
    (:`OnInterrupted`
      _)
    (:`OnCancelled`
      _))
  (`self.K2_EndAbility`)
  (`/Engine/EditorBlueprintResources/StandardMacros.IsValid` _braincomponent
    (:`Is Valid`
      (if (not (`GameplayTagAssetInterface.HasMatchingGameplayTag` (`AbilitySystemBlueprintLibrary.GetAbilitySystemComponent` (`self.GetAvatarActorFromActorInfo`)) (struct :`TagName` "State.Dead")))
        (bind _ascharacter_2 (cast `Character` (`self.GetAvatarActorFromActorInfo`)))
        (`CharacterMovementComponent.SetMovementMode` (`Character.CharacterMovement` _ascharacter_2) "MOVE_Walking" 0)
        (bind _asaicontroller_2 (cast `AIController` (`Pawn.GetController` _ascharacter_2)))
        (bind _braincomponent_2 (`AIController.BrainComponent` _asaicontroller_2))
        (`/Engine/EditorBlueprintResources/StandardMacros.IsValid` _braincomponent_2
          (:`Is Valid`
            (`BrainComponent.RestartLogic` _braincomponent_2)))))))