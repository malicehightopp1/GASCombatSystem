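; BP_PlayerCombatCharacter is the player's combat character Blueprint, adding keyboard shortcuts for switching weapons and quitting the game.
; Number keys 4 to 7 call EquipWeapon on the WeaponComponent, each passing a weapon data asset for unarmed, great hammer, dagger or longsword.
; Escape quits the game directly.
; BeginPlay, Tick, overlap and the construction script hold no logic.
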(event `Key|Escape`
  (params (Key :type "Key Structure"))
  (:`Pressed`
    (`KismetSystemLibrary.QuitGame` null "Quit")))

(event `Key|Four`
  (params (Key :type "Key Structure"))
  (:`Pressed`
    (`WeaponComponent.EquipWeapon` (`self.WeaponComponent`) "/Game/_MyFiles/Combat/WeaponData/DA_Unarmed.DA_Unarmed")))

(event `Key|Five`
  (params (Key :type "Key Structure"))
  (:`Pressed`
    (`WeaponComponent.EquipWeapon` (`self.WeaponComponent`) "/Game/_MyFiles/Combat/WeaponData/DA_GreatHammer.DA_GreatHammer")))

(event `Key|Six`
  (params (Key :type "Key Structure"))
  (:`Pressed`
    (`WeaponComponent.EquipWeapon` (`self.WeaponComponent`) "/Game/_MyFiles/Combat/WeaponData/DA_Dagger.DA_Dagger")))

(event `Key|Seven`
  (params (Key :type "Key Structure"))
  (:`Pressed`
    (`WeaponComponent.EquipWeapon` (`self.WeaponComponent`) "/Game/_MyFiles/Combat/WeaponData/DA_Longsword.DA_Longsword")))

(fn `UserConstructionScript`)