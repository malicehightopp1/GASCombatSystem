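; AI controller for enemy characters that drives the BT_Enemy behavior tree and reacts to perception of the player.
; On possess it starts the tree and stores the pawn's spawn position as HomeLocation in the blackboard.
; Perception updates for BP_PlayerCombatCharacter swap blackboard keys: TargetActor while sensed, LastKnownLocation from the stimulus when lost.
; Both transitions print debug messages.
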(event `self.ReceivePossess`
  (params (PossessedPawn :type "Pawn Object Reference"))
  (`self.RunBehaviorTree` "/Game/_MyFiles/Characters/EnemyAI/AIComponents/BT_Enemy.BT_Enemy")
  (`BlackboardComponent.SetValueAsVector` (`AIBlueprintHelperLibrary.GetBlackboard` null) (`self.HomeLocation`) (`self.K2_GetActorLocation` PossessedPawn)))

(event `self.AIPerception.OnTargetPerceptionUpdated`
  (params (Actor :type "Actor Object Reference") (Stimulus :type "AIStimulus Structure"))
  (bind (_age _expirationage _strength _stimuluslocation _receiverlocation _tag _bsuccessfullysensed) (break `AIStimulus` Stimulus))
  (bind _returnvalue (`AIBlueprintHelperLibrary.GetBlackboard` null))
  (bind _lastknownlocation (`self.LastKnownLocation`))
  (cast `/Game/_MyFiles/Characters/Player/BP_PlayerCombatCharacter` Actor)
  (if _bsuccessfullysensed
    (`BlackboardComponent.SetValueAsObject` _returnvalue (`self.TargetActor`) Actor)
    (`BlackboardComponent.ClearValue` _returnvalue _lastknownlocation)
    (`KismetSystemLibrary.PrintString` "SEEN PLAYER")
    (else
      (`BlackboardComponent.SetValueAsVector` _returnvalue _lastknownlocation _stimuluslocation)
      (`BlackboardComponent.ClearValue` _returnvalue (`self.TargetActor`))
      (`KismetSystemLibrary.PrintString` "LOST PLAYER"))))

(fn `UserConstructionScript`)