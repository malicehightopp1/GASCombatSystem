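; BP_TrainingDummy is a training dummy character that, as written, only prints debug values at game start.
; After a short delay on BeginPlay, it reads float attributes from itself through the Gameplay Ability System and prints them, showing each on screen only if the lookup succeeds.
; It then prints the Character Movement max walk speed, and has no other active logic.
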(event `self.ReceiveBeginPlay`
  (bind (_bsuccessfullyfoundattribute _returnvalue) (`AbilitySystemBlueprintLibrary.GetFloatAttribute` self (struct :`AttributeName` "MovementSpeed" :`Attribute` "/Script/CombatSystem.CombatAttributeSet:MovementSpeed" :`AttributeOwner` "/Script/CoreUObject.Class'/Script/CombatSystem.CombatAttributeSet'")))
  (bind (_bsuccessfullyfoundattribute_2 _returnvalue_2) (`AbilitySystemBlueprintLibrary.GetFloatAttribute` self (struct :`AttributeName` "Damage" :`Attribute` "/Script/CombatSystem.CombatAttributeSet:Damage" :`AttributeOwner` "/Script/CoreUObject.Class'/Script/CombatSystem.CombatAttributeSet'")))
  (`KismetSystemLibrary.Delay` 0.2)
  (`KismetSystemLibrary.PrintString` (`KismetStringLibrary.Conv_DoubleToString` _returnvalue) _bsuccessfullyfoundattribute)
  (`KismetSystemLibrary.PrintString` (`KismetStringLibrary.Conv_DoubleToString` _returnvalue_2) _bsuccessfullyfoundattribute_2)
  (`KismetSystemLibrary.PrintString` (`KismetStringLibrary.Conv_DoubleToString` (`CharacterMovementComponent.MaxWalkSpeed` (`self.CharacterMovement`)))))

(fn `UserConstructionScript`)